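; BP_ElevatorButton is a player-operated button that summons its linked elevator to the button's floor.
; The PlayerCatcher overlap tracks the player pawn, toggling input and a debug text as it enters and leaves.
; Pressing Interact inside plays a timeline that moves the button mesh along its local Z.
; When the timeline finishes, it activates the Elevator only if IsBaseFloor differs from the elevator's IsAtBaseLocation.
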(event OnComponentBeginOverlap(PlayerCatcher)
  (params (OverlappedComponent :type Primitive%20Component%20Object%20Reference) (OtherActor :type Actor%20Object%20Reference) (OtherComp :type Primitive%20Component%20Object%20Reference) (OtherBodyIndex :type Integer) (bFromSweep :type Boolean) (SweepResult :type Hit%20Result%20Structure%20%28by%20ref%29))
  ;[0 0 0] Check If Player is INside.
  (if (== OtherActor (Game|Player|GetPlayerPawn 0))
    (Variables|Default|SetPlayerIsInside true)
    (Development|SetHiddeninGame (Variables|Default|GetDebugText) false false)
    (Input|EnableInput (Game|GetPlayerController 0))))

(event OnComponentEndOverlap(PlayerCatcher)
  (params (OverlappedComponent :type Primitive%20Component%20Object%20Reference) (OtherActor :type Actor%20Object%20Reference) (OtherComp :type Primitive%20Component%20Object%20Reference) (OtherBodyIndex :type Integer))
  ;[0 0 0] Check If Player is INside.
  (if (== OtherActor (Game|Player|GetPlayerPawn 0))
    (Variables|Default|SetPlayerIsInside false)
    (Development|SetHiddeninGame (Variables|Default|GetDebugText) true false)
    (Input|DisableInput (Game|GetPlayerController 0))))

(event Custom|ActivateButton
  ;[0 0 0] Button Activation Timeline.
  (bind _alpha (Timeline|ButtonTimeline PlayFromStart)
    (:Update
      (Transformation|SetRelativeLocation (Variables|Default|GetButton) (Math|Vector|MakeVector 0.0 0.0 (Math|Float|Lerp 0.0 5.0 _alpha)) false false))
    (:Finished
      (CallFunction|ActivateElevator))))

(event Custom|ActivateElevator
  ;[0 0 0] Activate Elevator
  (if (not (== (Variables|Default|GetIsBaseFloor) (Variables|/Game/MUA/Environment/_Dev/BP_Elevator.BP_Elevator_C|GetIsAtBaseLocation (Variables|Default|GetElevator))))
    (Default|ActivateElevator (Variables|Default|GetElevator))))

(event EventBeginPlay
  ;[0.09446 0.8333 0] Begin Play
)

(event Collision|EventActorBeginOverlap
  (params (OtherActor :type Actor%20Object%20Reference)))

(event EventTick
  (params (DeltaSeconds :type Float%20%28single-precision%29)))

(event Input|ActionEvents|InputActionInteract
  (params (Key :type Key%20Structure :default "None"))
  ;[0 0 0] Activate Button
  (:Pressed
    (if (Variables|Default|GetPlayerIsInside)
      (CallFunction|ActivateButton))))

(fn ConstructionScript)