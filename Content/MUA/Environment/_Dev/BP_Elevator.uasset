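; Elevator platform actor that travels vertically between its base height and a target height when the player enters its catcher volume.
; A timeline lerps the mesh's relative Z, playing forward or in reverse depending on the current end, and ignores triggers while moving.
; The construction script copies the chosen mesh and rotation to a ghost component, whose height sets the target, and applies the speed as timeline play rate.
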(event OnComponentBeginOverlap(PlayerCatcher)
  (params (OverlappedComponent :type Primitive%20Component%20Object%20Reference) (OtherActor :type Actor%20Object%20Reference) (OtherComp :type Primitive%20Component%20Object%20Reference) (OtherBodyIndex :type Integer) (bFromSweep :type Boolean) (SweepResult :type Hit%20Result%20Structure%20%28by%20ref%29))
  (if (== OtherActor (Game|Player|GetPlayerPawn 0))
    (CallFunction|ActivateElevator)))

(event Custom|ActivateElevator
  (if (not (Variables|Default|GetIsMoving))
    (Variables|Default|SetIsMoving true)
    (if (Variables|Default|GetIsAtBaseLocation)
      (bind (_direction _alpha) (Timeline|ElevatorTimeline PlayFromStart)
        (:Update
          (Transformation|SetRelativeLocation (Variables|Default|GetBase) (Math|Vector|MakeVector 0.0 0.0 (Math|Float|Lerp (Variables|Default|GetBaseElevation) (Variables|Default|GetTargetElevation) _alpha)) false false))
        (:Finished
          (switch Utilities|FlowControl|Switch|SwitchonETimelineDirection _direction
            (:Forward
              (Variables|Default|SetIsAtBaseLocation false))
            (:Backward
              (Variables|Default|SetIsAtBaseLocation true)))
          (Variables|Default|SetIsMoving false)))
      (else
        (Timeline|ElevatorTimeline ReverseFromEnd)))))

(event EventBeginPlay
  (Variables|Default|SetTargetElevation (.z (.location (Transformation|GetRelativeTransform (Variables|Default|GetTargetGhost)))))
  (Input|EnableInput (Game|GetPlayerController 0)))

(fn ConstructionScript
  (bind _targetghost (Variables|Default|GetTargetGhost))
  (bind _base (Variables|Default|GetBase))
  (Components|StaticMesh|SetStaticMesh _base (Variables|ElevatorSettings|GetElevatorMesh))
  (Components|StaticMesh|SetStaticMesh _targetghost (Variables|/Script/Engine.StaticMeshComponent|GetStaticMesh (Variables|Default|GetBase)))
  (Transformation|SetRelativeRotation _targetghost (Variables|/Script/Engine.SceneComponent|GetRelativeRotation _base) false false)
  (Components|Timeline|SetPlayRate (Variables|Default|GetElevatorTimeline) (Variables|ElevatorSettings|GetElevatorSpeed)))