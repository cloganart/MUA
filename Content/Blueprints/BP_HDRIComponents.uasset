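; BP_HDRIComponents is an HDRI environment actor whose sky dome and background mesh image rotation follows the actor's yaw.
; When both materials are valid, the Construction Script reads the starting "Rotation" parameter from the sky dome material.
; It then creates dynamic material instances for both meshes and sets their "Rotation" to that start value plus the root's yaw, normalized to turns and negated.
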(event EventBeginPlay)

(event Collision|EventActorBeginOverlap
  (params (OtherActor :type Actor%20Object%20Reference)))

(event EventTick
  (params (DeltaSeconds :type Float%20%28single-precision%29)))

(fn ConstructionScript
  (bind _skydomematerial (Variables|Default|GetSkyDomeMaterial))
  (bind _backgroundmaterial (Variables|Default|GetBackgroundMaterial))
  (bind _skydome (Variables|Default|GetSkyDome))
  (bind _background (Variables|Default|GetBackground))
  (if (and (Utilities|IsValid _skydomematerial) (Utilities|IsValid _backgroundmaterial))
    (Utilities|FlowControl|Sequence
      (:then_0
        (for _array_element (Variables|/Script/Engine.MaterialInstance|GetScalarParameterValues _skydomematerial)
          (if (Utilities|Name|Equal(Name) (.name (.parameterinfo _array_element)) "Rotation")
            (Variables|Default|SetHDRIStartRotation (.parametervalue _array_element)))))
      (:then_1
        (Rendering|Material|SetMaterial _skydome 0 _skydomematerial)
        (Rendering|Material|SetMaterial _background 0 _backgroundmaterial)
        (bind _returnvalue (Rendering|Material|CreateDynamicMaterialInstance _skydome 0 _skydomematerial "None" :!class /Script/Engine.PrimitiveComponent))
        (Variables|Default|SetSkyDomeMID _returnvalue)
        (bind _returnvalue_2 (Rendering|Material|CreateDynamicMaterialInstance _background 0 _backgroundmaterial "None" :!class /Script/Engine.PrimitiveComponent))
        (bind _output_get (Variables|Default|SetBackgroundMeshMID _returnvalue_2))
        (Rendering|Material|GetScalarParameterValue _output_get "Rotation" :!class /Script/Engine.MaterialInstanceDynamic)
        (Rendering|Material|SetScalarParameterValue (Variables|Default|GetBackgroundMeshMID) "Rotation" (+ (Variables|Default|GetHDRIStartRotation) (/ (.yaw (Transformation|GetWorldRotation (Variables|Default|GetDefaultSceneRoot))) -3.6e+02)) :!class /Script/Engine.MaterialInstanceDynamic)
        (Rendering|Material|SetScalarParameterValue (Variables|Default|GetSkyDomeMID) "Rotation" (+ (Variables|Default|GetHDRIStartRotation) (/ (.yaw (Transformation|GetWorldRotation (Variables|Default|GetDefaultSceneRoot))) -3.6e+02)) :!class /Script/Engine.MaterialInstanceDynamic)))))